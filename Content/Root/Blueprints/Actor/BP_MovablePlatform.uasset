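; BP_MovablePlatform is an actor that moves vertically between its starting location and a point offset by ZDelta on the Z axis.
; On BeginPlay it caches both endpoints, waits a random fraction of a second, then plays a Timeline whose alpha lerps the actor's location without sweeping.
; The Timeline's play rate is the inverse of a random float, so each instance varies in start time and speed.
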(event EventBeginPlay
  (bind _timeline (Variables|Default|GetTimeline))
  (Variables|Default|SetStart%20Location (Transformation|GetActorLocation))
  (Variables|Default|SetTarget%20Location (+ (Variables|Default|GetStart%20Location) (Math|Vector|MakeVector 0.0 0.0 (Variables|Default|GetZ-Delta))))
  (Utilities|FlowControl|Delay (Math|Random|RandomFloat))
  (Components|Timeline|SetPlayRate _timeline (/ 1.0 (Math|Random|RandomFloat)))
  (Audio|Components|Audio|Play _timeline))

(event Collision|EventActorBeginOverlap
  (params (OtherActor :type Actor%20Object%20Reference)))

(event EventTick
  (params (DeltaSeconds :type Float%20%28single-precision%29)))

(fn ConstructionScript)