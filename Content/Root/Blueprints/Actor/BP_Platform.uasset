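; BP_Platform is a platform actor whose Cube component becomes physics-driven while the player is overlapping it.
; On actor begin overlap it checks for player character 0 and enables physics simulation on the Cube, then disables it again on end overlap.
; Tick and the construction script are empty, and unconnected vector math involving a LaunchPower variable and the player's forward vector is left unused.
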(event Collision|EventActorBeginOverlap
  (params (OtherActor :type Actor%20Object%20Reference))
  (if (== OtherActor (Game|GetPlayerCharacter 0))
    (Physics|SetSimulatePhysics (Variables|Default|GetCube) true)))

(event Collision|EventActorEndOverlap
  (params (OtherActor :type Actor%20Object%20Reference))
  (if (== OtherActor (Game|GetPlayerCharacter 0))
    (Physics|SetSimulatePhysics (Variables|Default|GetCube) false)))

(event EventTick
  (params (DeltaSeconds :type Float%20%28single-precision%29)))

(fn ConstructionScript)