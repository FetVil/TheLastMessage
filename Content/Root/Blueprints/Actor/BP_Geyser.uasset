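; BP_Geyser is a geyser actor that switches on and off periodically and pushes overlapping platforms while active.
; Each tick while Status is on, it applies a force to the Cube of every overlapping BP_Platform, mapping WindTo onto world X and Z, scaled by LaunchPower.
; A Timer-length Delay on the same Tick flips Status and shows or hides the geyser's own Cube to match.
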(event EventTick
  (params (DeltaSeconds :type Float%20%28single-precision%29))
  (bind _windto (Variables|Default|GetWindTo))
  (Utilities|FlowControl|Sequence
    (:then_0
      (if (Variables|Default|GetStatus)
        (for _array_element (Collision|GetOverlappingActors "/Game/Root/Blueprints/Actor/BP_Platform.BP_Platform_C" :!class /Script/Engine.Actor)
          (Physics|AddForce (Variables|/Game/Root/Blueprints/Actor/BP_Platform.BP_Platform_C|GetCube _array_element) (* (Math|Vector|MakeVector (.x _windto) 0.0 (.y _windto)) (Variables|Default|GetLaunchPower)) "None" false))))
    (:then_1
      (Utilities|FlowControl|Delay (Variables|Default|GetTimer))
      (if (Variables|Default|GetStatus)
        (Variables|Default|SetStatus false)
        (Development|SetHiddeninGame (Variables|Default|GetCube) true false)
        (else
          (Variables|Default|SetStatus true)
          (Development|SetHiddeninGame (Variables|Default|GetCube) false false))))))

(fn ConstructionScript)