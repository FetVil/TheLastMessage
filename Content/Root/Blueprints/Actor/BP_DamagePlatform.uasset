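; BP_DamagePlatform is a platform actor that launches characters upward; despite its name, it applies no damage.
; Each Tick loops over overlapping Characters and, if the begin-overlap event's OtherActor is the player, adds upward launch velocity to both the player and the looped character.
; The begin-overlap event runs no logic itself, and nodes for LaunchPower scaling and player location are left unused.
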(event Collision|EventActorBeginOverlap
  (params (OtherActor :type Actor%20Object%20Reference)))

(event EventTick
  (params (DeltaSeconds :type Float%20%28single-precision%29))
  (bind _returnvalue (Game|GetPlayerCharacter 0))
  (for _array_element (Collision|GetOverlappingActors "/Script/Engine.Character" :!class /Script/Engine.Actor)
    (if (== (stale Collision|EventActorBeginOverlap OtherActor) _returnvalue)
      (Character|LaunchCharacter _returnvalue (+ "" "0.000000,0.000000,200.000000") false false))))

(fn ConstructionScript)